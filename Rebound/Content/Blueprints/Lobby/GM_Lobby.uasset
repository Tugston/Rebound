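; Lobby game mode that sets up joining players, shares map settings and player lists, and starts the match by server travel.
; On authority, PostLogin records each controller, initializes its PC_Lobby menu from GameInfoInstance, then spawns a FirstPersonCharacter at a random PlayerStart.
; Respawns and settings changes push updates to every PC_Lobby.
; LaunchGame travels to TestMap when allowed; character swap and kick-list events are empty stubs.
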(event Custom|ReSpawnPlayer
  (params (Player%20Controller :type Player%20Controller%20Object%20Reference))
  (bind _returnvalue (Pawn|GetControlledPawn Player%20Controller))
  (bind _spawnpoints (Variables|ServerSettings|GetSpawnPoints))
  ;[1 1 1] Spawn the Player as their Character, Updates Lobby for Everyone
  (Utilities|IsValid _returnvalue
    (:Is%20Valid
      (Actor|DestroyActor _returnvalue)
      (Utilities|FlowControl|Delay 2.0))
    (:Is%20Not%20Valid
      _))
  (bind _returnvalue_2 (Game|SpawnActorfromClass "/Game/FirstPerson/FirstPersonBP/Blueprints/FirstPersonCharacter.FirstPersonCharacter_C" (Transformation|GetActorTransform (Utilities|Array|Get(acopy) _spawnpoints (Math|Random|RandomIntegerinRange 0 (- (Utilities|Array|Length _spawnpoints) 1)))) "Undefined" 0 0))
  (Pawn|Possess Player%20Controller _returnvalue_2)
  (CallFunction|EveryoneUpdate))

(event Custom|SwapCharacter
  (params (Controller :type Player%20Controller%20Object%20Reference) (Character%20Class :type Character%20Class%20Reference) (ChangedStatus :type Boolean)))

(event Custom|EveryoneUpdate
  (bind _allplayercontrollers (Variables|ServerSettings|GetAllPlayerControllers))
  ;[1 1 1] Updates All Connected Players Lobby Info
  (bind _output_get (Variables|ServerSettings|SetCurrentPlayers (Utilities|Array|Length (Variables|ServerSettings|GetAllPlayerControllers))))
  (if (> _output_get 0)
    (Utilities|Array|Clear (Variables|ServerSettings|GetConnectedPlayers))
    (for _array_element _allplayercontrollers
      (bind _aspc_lobby (Utilities|Casting|CastToPC_Lobby _array_element))
      (Utilities|Array|Add (Variables|ServerSettings|GetConnectedPlayers) (Variables|/Game/Blueprints/Lobby/PC_Lobby.PC_Lobby_C|GetPlayerSettings _aspc_lobby))
      (Default|UpdateNumberOfPlayers _aspc_lobby (Variables|ServerSettings|GetCurrentPlayers) (Variables|ServerSettings|GetMaxPlayers)))
    (for _array_element_2 _allplayercontrollers
      (bind _aspc_lobby_2 (Utilities|Casting|CastToPC_Lobby _array_element_2))
      (Default|AddPlayerInfo _aspc_lobby_2 (Variables|ServerSettings|GetConnectedPlayers))
      (CallFunction|AddtoKickList))))

(event Custom|LaunchGame
  (params (CanStart :type Boolean))
  ;[1 1 1] Launch The Game Based on Map Selection from Game Settings, If Everyone is Ready
  (if CanStart
    (switch int (Variables|ServerSettings|GetGM_MapID)
      (:0
        (Development|ExecuteConsoleCommand "servertravel /Game/Maps/TestMap" (Game|GetPlayerController 0))
        (Development|PrintString "Starting Game")))))

(event Custom|AddToKickList)

(event Custom|ServerUpdateGameSettings
  (params (MapImage :type Texture%202D%20Object%20Reference) (MapName :type Text) (MapTime :type Text) (mapID :type Integer))
  ;[1 1 1] Server Made Changes, Update Lobby Information for Everyone
  (Variables|ServerSettings|SetGM_MapImage MapImage)
  (Variables|ServerSettings|SetGM_MapName MapName)
  (Variables|ServerSettings|SetGM_MapTime MapTime)
  (Variables|ServerSettings|SetGM_MapID mapID)
  (for _array_element (Variables|ServerSettings|GetAllPlayerControllers)
    (bind _aspc_lobby (Utilities|Casting|CastToPC_Lobby _array_element))
    (Default|UpdateLobbySettings _aspc_lobby (Variables|ServerSettings|GetGM_MapImage) (Variables|ServerSettings|GetGM_MapName) (Variables|ServerSettings|GetGM_MapTime))))

(event EventPostLogin
  (params (NewPlayer :type Player%20Controller%20Object%20Reference))
  ;[1 1 1] Initial Setup, Occurs on Post Login, Handles Lobby Setup on Player Controller and Spawns Player
  (Networking|SwitchHasAuthority
    (:Authority
      (Utilities|Array|Add (Variables|ServerSettings|GetAllPlayerControllers) NewPlayer)
      (bind _outactors (Actor|GetAllActorsOfClass "/Script/Engine.PlayerStart"))
      (Variables|ServerSettings|SetSpawnPoints _outactors)
      (bind _asgame_info_instance (Utilities|Casting|CastToGameInfoInstance (Game|GetGameInstance)))
      (Variables|ServerSettings|SetServerName (Variables|/Game/Blueprints/MultiplayerItems/GameInfoInstance.GameInfoInstance_C|GetServerName _asgame_info_instance))
      (Variables|ServerSettings|SetMaxPlayers (Variables|/Game/Blueprints/MultiplayerItems/GameInfoInstance.GameInfoInstance_C|GetMaxPlayers _asgame_info_instance))
      (bind _aspc_lobby (Utilities|Casting|CastToPC_Lobby NewPlayer))
      (Default|InitialSetup _aspc_lobby)
      (Default|SetupLobbyMenu _aspc_lobby (Variables|ServerSettings|GetServerName))
      (Default|UpdateLobbySettings _aspc_lobby (Variables|ServerSettings|GetGM_MapImage) (Variables|ServerSettings|GetGM_MapName) (Variables|ServerSettings|GetGM_MapTime))
      (CallFunction|ReSpawnPlayer NewPlayer))))

(fn ConstructionScript)